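; BP_LDEnemySpawner launches an enemy along a Level Sequence once its Activate flag is set.
; Tick polls the flag, then creates and plays a player for EnemySequence, whose validity stops further triggering.
; If EnemyCourse is valid, it spawns a BP_LDEnemy there and attaches it to that actor, snapping location and scale while keeping world rotation.
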(event `self.ReceiveTick`
  (params (DeltaSeconds :type "Float (single-precision)"))
  (bind _enemycourse (`self.EnemyCourse`))
  (`/Engine/EditorBlueprintResources/StandardMacros.IsValid` (`self.EnemySequencePlayer`)
    (:`Is Not Valid`
      (if (`self.Activate`)
        (bind _returnvalue (`LevelSequencePlayer.CreateLevelSequencePlayer` self (`self.EnemySequence`) (make `LevelSequencePlaybackSettings` 0 1.0)))
        (bind _output_get (set `self.EnemySequencePlayer` _returnvalue))
        (`LevelSequencePlayer.Play` _output_get)
        (`/Engine/EditorBlueprintResources/StandardMacros.IsValid` _enemycourse
          (:`Is Valid`
            (bind _returnvalue_2 (`|SpawnActorFromClass` "/Game/LylatDragoon/Assets/Blueprints/BP_LDEnemy.BP_LDEnemy_C" (`self.GetTransform` _enemycourse) "Undefined" "OverrideRootScale" self))
            (`self.K2_AttachToActor` _returnvalue_2 _enemycourse "None" "SnapToTarget" "KeepWorld" "SnapToTarget" false)))))))

(fn `UserConstructionScript`)